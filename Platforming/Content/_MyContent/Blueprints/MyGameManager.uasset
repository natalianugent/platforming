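; MyGameManager tracks the game state (Running, Won, Lost or Abandon) and switches the matching UI screen.
; Init creates the result and instructions widgets, then enters Running.
; SetState hides the UI, then either hides the mouse or shows that state's widget with the cursor.
; ResetGame moves the player to the first PlayerStart and reruns Init, which creates the widgets again; ShowHUD is an empty stub.
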(event EventBeginPlay)

(event Collision|EventActorBeginOverlap
  (params (OtherActor :type Actor%20Object%20Reference)))

(event EventTick
  (params (DeltaSeconds :type Float%20%28single-precision%29)))

(fn ConstructionScript)

(fn Init
  (CallFunction|CreateUI)
  (CallFunction|SetState "NewEnumerator0"))

(fn SetState
  (params (New%20State :type MyGameStates%20Enum :default "NewEnumerator0"))
  (CallFunction|HideUI)
  (bind _output_get (Variables|Default|SetCurrent%20Game%20State New%20State))
  (switch Utilities|FlowControl|Switch|SwitchonMyGameStates _output_get
    (:NewEnumerator0
      (CallFunction|ShowMouse false)
      (CallFunction|ShowHUD false))
    (:NewEnumerator1
      (Widget|SetVisibility (Variables|Default|GetWidget_Won) "Visible")
      (CallFunction|ShowMouse true :!label _label))
    (:NewEnumerator2
      (Widget|SetVisibility (Variables|Default|GetWidget_Lost) "Visible")
      (goto _label))
    (:NewEnumerator3
      (Widget|SetVisibility (Variables|Default|GetWidget_Abandon) "Visible")
      (goto _label))))

(fn GetState
  (return (Variables|Default|GetCurrent%20Game%20State)))

(fn CreateUI
  (bind _returnvalue (UserInterface|CreateWidget "/Game/_MyContent/UI/Widget_Abandon.Widget_Abandon_C"))
  (bind _output_get (Variables|Default|SetWidget_Abandon _returnvalue))
  (UserInterface|Viewport|AddtoViewport _output_get 0)
  (bind _returnvalue_2 (UserInterface|CreateWidget "/Game/_MyContent/UI/Widget_Won.Widget_Won_C"))
  (bind _output_get_2 (Variables|Default|SetWidget_Won _returnvalue_2))
  (UserInterface|Viewport|AddtoViewport _output_get_2 0)
  (bind _returnvalue_3 (UserInterface|CreateWidget "/Game/_MyContent/UI/Widget_Lost.Widget_Lost_C"))
  (bind _output_get_3 (Variables|Default|SetWidget_Lost _returnvalue_3))
  (UserInterface|Viewport|AddtoViewport _output_get_3 0)
  (bind _returnvalue_4 (UserInterface|CreateWidget "/Game/_MyContent/UI/Widget_Instructions.Widget_Instructions_C"))
  (bind _output_get_4 (Variables|Default|SetWidget%20Intructions _returnvalue_4))
  (UserInterface|Viewport|AddtoViewport _output_get_4 0))

(fn ResetGame
  (bind _outactors (Actor|GetAllActorsOfClass "/Script/Engine.PlayerStart"))
  (Transformation|SetActorLocation (Variables|Default|GetMy%20Player) (Transformation|GetActorLocation (Utilities|Array|Get(acopy) _outactors)) false false)
  (bind _my_game_manager (CallFunction|GetMyGameManager))
  (CallFunction|Init _my_game_manager))

(fn ShowHUD
  (params (Visable :type Boolean)))